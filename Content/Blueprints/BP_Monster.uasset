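; BP_Monster is an enemy, animated as a bear, with a health bar widget that appears when the player is near.
; BeginPlay hides the widget and hands the monster reference to its WBP_HPBar.
; Sphere overlaps with BP_MyPlayer show and hide the bar.
; DeadAnim disables capsule and mesh collision, plays the death montage and destroys the actor whether the montage completes or is interrupted.
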(event `self.ReceiveBeginPlay`
  (bind _widget (`self.Widget`))
  (`SceneComponent.SetVisibility` _widget false false)
  (bind _aswbp_hpbar (cast `/Game/Blueprints/Widget/WBP_HPBar` (`WidgetComponent.GetWidget` _widget)))
  (set `/Game/Blueprints/Widget/WBP_HPBar.As BP Monster` self _aswbp_hpbar))

(event `self.DeadAnim`
  (`PrimitiveComponent.SetCollisionEnabled` (`self.CapsuleComponent`) "NoCollision")
  (`PrimitiveComponent.SetCollisionEnabled` (`self.Mesh`) "NoCollision")
  (`|PlayMontage` (`self.Mesh`) "/Game/InfinityBladeAdversaries/Enemy/Enemy_Bear/Enemy_Bear_Animations/Bear_Death_Montage.Bear_Death_Montage"
    (:`OnCompleted`
      _)
    (:`OnInterrupted`
      _))
  (`self.K2_DestroyActor`))

(event `self.Sphere.OnComponentBeginOverlap`
  (params (OverlappedComponent :type "PrimitiveComponent Object Reference") (OtherActor :type "Actor Object Reference") (OtherComp :type "PrimitiveComponent Object Reference") (OtherBodyIndex :type Integer) (bFromSweep :type Boolean) (SweepResult :type "HitResult Structure (by ref)"))
  (cast `/Game/Blueprints/BP_MyPlayer` OtherActor)
  (`SceneComponent.SetVisibility` (`self.Widget`) true false))

(event `self.Sphere.OnComponentEndOverlap`
  (params (OverlappedComponent :type "PrimitiveComponent Object Reference") (OtherActor :type "Actor Object Reference") (OtherComp :type "PrimitiveComponent Object Reference") (OtherBodyIndex :type Integer))
  (cast `/Game/Blueprints/BP_MyPlayer` OtherActor)
  (`SceneComponent.SetVisibility` (`self.Widget`) false false))

(fn `UserConstructionScript`)